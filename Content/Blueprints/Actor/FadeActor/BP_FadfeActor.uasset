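; Fadeable mesh actor that fades out and back in through its materials when FadeOut or Fadein is called.
; On BeginPlay it creates dynamic instances of the mesh's materials, and a timeline played forward or in reverse drives their AAMaskValue parameter.
; When the timeline finishes, the fade value switches a custom trace channel response to Overlap (if BlockVisablity is set) or Ignore.
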(event EventBeginPlay
  (CallFunction|SetupDynamicMaterial))

(event Collision|EventActorBeginOverlap
  (params (OtherActor :type Actor%20Object%20Reference)))

(event EventTick
  (params (DeltaSeconds :type Float%20%28single-precision%29)))

(event EventFadein
  (bind _fade (Timeline|FadeLerp Reverse)
    (:Update
      (Variables|Default|SetFadeValue _fade)
      (CallFunction|UpdataFade))
    (:Finished
      (CallFunction|ChangeMeshVisbilityCollision))))

(event EventFadeOut
  (bind _fade (Timeline|FadeLerp Play)
    (:Update
      (Variables|Default|SetFadeValue _fade)
      (CallFunction|UpdataFade))
    (:Finished
      (CallFunction|ChangeMeshVisbilityCollision))))

(fn ConstructionScript)

(fn UpdataFade
  (for (_array_element _array_index) (Variables|Default|GetDynamicMaterial)
    (Rendering|Material|SetMaterial (Variables|Default|GetMesh) _array_index _array_element)
    (Rendering|Material|SetScalarParameterValue (Utilities|Array|Get(acopy) (Variables|Default|GetDynamicMaterial) _array_index) "AAMaskValue" (Variables|Default|GetFadeValue) :!class /Script/Engine.MaterialInstanceDynamic)))

(fn ChangeMeshVisbilityCollision
  (bind _fadevalue (Variables|Default|GetFadeValue))
  (if (>= _fadevalue 0.99)
    (if (Variables|Default|GetbBlockVisablity)
      (Collision|SetCollisionResponsetoChannel (Variables|Default|GetMesh) "ECC_GameTraceChannel2" "ECR_Overlap"))
    (elif (<= _fadevalue 0.41)
      (Collision|SetCollisionResponsetoChannel (Variables|Default|GetMesh) "ECC_GameTraceChannel2" "ECR_Ignore"))))

(fn SetupDynamicMaterial
  (Utilities|Array|Clear (Variables|Default|GetDynamicMaterial))
  (bind _output_get (Variables|Default|SetMeshOriginalMaterials (Rendering|Material|GetMaterials (Variables|Default|GetMesh))))
  (for _array_element _output_get
    (bind _returnvalue (Rendering|Material|CreateDynamicMaterialInstance _array_element "None" "None" :!class /Script/Engine.KismetMaterialLibrary))
    (Utilities|Array|AddUnique (Variables|Default|GetDynamicMaterial) _returnvalue)))