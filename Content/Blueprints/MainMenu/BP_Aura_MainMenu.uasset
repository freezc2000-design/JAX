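; Main menu display actor for Aura that sets up the menu screen and animates a floating fire component.
; On BeginPlay it plays menu music, adds WBP_MainMenu to the viewport and shows the mouse cursor.
; It then caches the fire's start position and a slightly raised end point, and the Cycle timeline lerps the fire between them.
; The UI-only input mode call is left unconnected, so it never runs.
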(event EventBeginPlay
  (Utilities|FlowControl|Sequence
    (:then_0
      (Audio|PlaySound2D "/Game/Assets/Sounds/Music/Music_MainMenu.Music_MainMenu" 1.0 1.0 0.0 0 0)
      (bind _returnvalue (UserInterface|CreateWidget "/Game/Blueprints/UI/MainMenu/WBP_MainMenu.WBP_MainMenu_C"))
      (UserInterface|Viewport|AddtoViewport _returnvalue 0)
      (Variables|/Script/Engine.PlayerController|SetbShowMouseCursor (Game|GetPlayerController 0) true))
    (:then_1
      (CallFunction|初始化火球位移)
      (bind _alpha (Timeline|Cycle PlayFromStart)
        (:Update
          (Transformation|SetWorldLocation (Variables|Default|GetFire) (Math|Vector|Lerp(Vector) (Variables|Default|GetBeginLocation) (Variables|Default|GetEndLocation) _alpha) false false))))))

(event Collision|EventActorBeginOverlap
  (params (OtherActor :type Actor%20Object%20Reference)))

(event EventTick
  (params (DeltaSeconds :type Float%20%28single-precision%29)))

(fn ConstructionScript)

(fn 初始化火球位移
  (bind _output_get (Variables|Default|SetBeginLocation (Transformation|GetWorldLocation (Variables|Default|GetFire))))
  (Variables|Default|SetEndLocation (+ _output_get (* (Transformation|GetActorUpVector) 1e+01))))