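; Enemy ranged attack Gameplay Ability that fires a projectile at the avatar's current combat target.
; Through CombatInterface it turns the avatar toward the target and plays a random tagged attack montage, ending early if target or interface is missing.
; A gameplay event matching the montage's SocketTag triggers SpawnProjectile at the target's location, with optional pitch override.
; The ability ends when the montage completes, is interrupted or is cancelled.
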(event Ability|EventActivateAbility
  (bind _returnvalue (Ability|GetAvatarActorfromActorInfo))
  (bind _returnvalue_2 (Class|CombatInterface|GetCombatTarget(Message) _returnvalue))
  (bind _ascombat_interface (Utilities|Casting|CastToCombatInterface _returnvalue)
    (:then
      (Utilities|IsValid _returnvalue_2
        (:Is%20Valid
          (Class|CombatInterface|SetFaceingTargetLoc _ascombat_interface (Transformation|GetActorLocation _returnvalue_2))
          (bind _returnvalue_3 (Class|CombatInterface|GetAttackMontages(Message) (Ability|GetAvatarActorfromActorInfo)))
          (bind _output_get (Variables|Default|SetSlecetedMontage (Class|AuraDamageGameplayAbility|GetRandomTaggedMontage _returnvalue_3)))
          (|PlayMontageandWaitProxy "None" (.montage _output_get) 1.0 "None" false 1.0 0.0 false
            (:then
              (Ability|Tasks|WaitGameplayEvent (.sockettag _output_get) 0 true
                (:EventReceived
                  (Class|AuraProjectileSpell|SpawnProjectile (Transformation|GetActorLocation _returnvalue_2) (Variables|Default|GetbShouldOverridePitch) (Variables|Default|GetPitch%20OverrideDeg)))))
            (:OnCompleted
              (Ability|EndAbility :!label _label))
            (:OnInterrupted
              (goto _label))
            (:OnCancelled
              (goto _label))))
        (:Is%20Not%20Valid
          (Ability|EndAbility :!label _label_2))))
    (:CastFailed
      (goto _label_2))))

(event Ability|EventOnEndAbility
  (params (bWasCancelled :type Boolean)))