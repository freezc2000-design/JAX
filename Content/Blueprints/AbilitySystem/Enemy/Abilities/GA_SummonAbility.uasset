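; Enemy shaman Gameplay Ability that faces the combat target and summons random minions at shuffled spawn locations.
; It plays a summon montage, shows ground Niagara effects at every location, then waits for the montage's attack gameplay event.
; A delayed loop spawns each minion with its default controller.
; The avatar's minion count rises by Index + 1 afterward and drops on each minion's destruction; EndAbility is never reached.
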(event Custom|OnDestroyed_Event
  (params (DestroyedActor :type Actor%20Object%20Reference))
  ;[1 1 1] 死亡时召唤物计数减少
  (Class|CombatInterface|IncrementMinionCount(Message) (Ability|GetAvatarActorfromActorInfo) -1))

(event Ability|EventActivateAbility
  (bind _returnvalue (Ability|GetAvatarActorfromActorInfo))
  (bind _index (Variables|Default|GetIndex))
  (bind _returnvalue_2 (Class|CombatInterface|GetCombatTarget(Message) _returnvalue))
  (Class|CombatInterface|SetFaceingTargetLoc(Message) _returnvalue (Transformation|GetActorLocation _returnvalue_2))
  (|PlayMontageandWaitProxy "None" "/Game/Characters/Enemies/Art/Shaman/Animations/AM_Shaman_Summon.AM_Shaman_Summon" 1.0 "None" true 1.0 0.0 false
    (:then
      (Utilities|FlowControl|Delay 0.2)
      (bind _returnvalue_3 (Class|AuraSummonAbility|GetSpwanLocation))
      (Utilities|Array|Shuffle _returnvalue_3)
      (for _array_element _returnvalue_3
        (Niagara|SpawnSystematLocation "/Game/Assets/Effects/Combat/NS_GroundSummon.NS_GroundSummon" _array_element))
      (Ability|Tasks|WaitGameplayEvent "(TagName=\"Montage.Attack.1\")" (Ability|GetAvatarActorfromActorInfo)
        (:EventReceived
          (if (<= _index (Utilities|Array|LastIndex _returnvalue_3)) :!label _label
            (bind _returnvalue_4 (Game|SpawnActorfromClass (Class|AuraSummonAbility|GetRandomMinionClass) (Math|Transform|MakeTransform (+ (Utilities|Array|Get(acopy) _returnvalue_3 _index) "0.000000,0.000000,20.000000") (Transformation|GetActorRotation (Ability|GetAvatarActorfromActorInfo)) "1.000000,1.000000,1.000000") "AdjustIfPossibleButAlwaysSpawn" "MultiplyWithRoot" 0 0))
            (Game|AssignOnDestroyed _returnvalue_4 (delegate Custom|OnDestroyed_Event))
            (bind _aspawn (Utilities|Casting|CastToPawn _returnvalue_4)
              (:then
                (Pawn|SpawnDefaultController _aspawn))
              (:CastFailed
                _))
            (Math|Integer|IncrementInt (Variables|Default|GetIndex)
              (:%20%20
                (Utilities|FlowControl|Delay 0.4)
                (goto _label)))
            (else
              (Class|CombatInterface|IncrementMinionCount(Message) (Ability|GetAvatarActorfromActorInfo) (+ (Variables|Default|GetIndex) 1)))))))))

(event Ability|EventOnEndAbility
  (params (bWasCancelled :type Boolean)))