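; GA_AutoOrb is an Aura gameplay ability whose event graph is inert: no activation event drives its logic, and OnEndAbility is empty.
; The disconnected chain takes the target under the mouse, turns the avatar toward it, plays the FireBolt cast montage, then on its gameplay event commits and spawns homing projectiles.
; Stray single-projectile and EndAbility nodes remain, the latter noting that an immediate server-side end stops clients receiving the trigger.
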(event Ability|EventOnEndAbility
  (params (bWasCancelled :type Boolean)))