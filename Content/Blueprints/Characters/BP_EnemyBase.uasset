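; Base enemy character Blueprint providing spawn, dissolve and loot-drop behavior.
; A timeline scales the actor at BeginPlay for a bouncy pop, and two others drive the Dissolve parameter on mesh and weapon materials.
; A FacingTarget motion-warp point orients the enemy toward given locations.
; Loot rolled from loot tiers spawns one item per looping timer tick in an evenly spaced ring at random distances, passing the enemy's level to effect actors.
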(event Custom|SpawnLootItem
  ;[1 1 1] 生成掉落物
  (bind _returnvalue (Game|SpawnActorfromClass (.LootClass (Utilities|Struct|BreakLootItem (Utilities|Array|Get(acopy) (Variables|Default|GetPureSpawnItem) (Variables|Default|GetSpawnedLootCount)))) (CallFunction|GetSpawnTransfrom (Math|Random|RandomFloatinRange 5e+01 1.5e+02)) "AdjustIfPossibleButAlwaysSpawn" "MultiplyWithRoot" 0 0))
  (bind _asaura_effect_actor (Utilities|Casting|CastToAuraEffectActor _returnvalue)
    (:then
      (Utilities|IsValid _asaura_effect_actor
        (:Is%20Valid
          (Variables|/Script/Aura_Learn.AuraEffectActor|SetActorLevel _asaura_effect_actor (Math|Conversions|ToFloat(Integer) (Variables|Default|GetLevel))))
        (:Is%20Not%20Valid
          _)))
    (:CastFailed
      _))
  (Math|Integer|IncrementInt (Variables|Default|GetSpawnedLootCount)
    (:%20%20
      (if (not (< (Variables|Default|GetSpawnedLootCount) (Utilities|Array|Length (Variables|Default|GetPureSpawnItem))))
        (Utilities|Time|ClearandInvalidateTimerbyHandle (Variables|Default|GetSpawnLootEventHandle))))))

(event EventBeginPlay
  (|CallParentFunction)
  ;[1 1 1] 通过缩放模型营造弹跳感
  (bind _scalvalue (Timeline|ScalPop Play)
    (:Update
      (Transformation|SetActorScale3D (Math|Conversions|ToVector(Float) _scalvalue)))))

(event Collision|EventActorBeginOverlap
  (params (OtherActor :type Actor%20Object%20Reference)))

(event EventTick
  (params (DeltaSeconds :type Float%20%28single-precision%29)))

(event EventStartDissolveTimlineOfMesh
  (params (DynamicMaterialInstance :type Material%20Instance%20Dynamic%20Object%20Reference))
  (bind _dissolve (Timeline|DissolveTimelineOfMesh Play)
    (:Update
      (Rendering|Material|SetScalarParameterValue DynamicMaterialInstance "Dissolve" _dissolve :!class /Script/Engine.MaterialInstanceDynamic))))

(event EventStartDissolveTimlineOfWeapon
  (params (DynamicMaterialInstance :type Material%20Instance%20Dynamic%20Object%20Reference))
  (bind _dissolve (Timeline|DissolveTimelineOfWeapon Play)
    (:Update
      (Rendering|Material|SetScalarParameterValue DynamicMaterialInstance "Dissolve" _dissolve :!class /Script/Engine.MaterialInstanceDynamic))))

(event EventSetFaceingTargetLoc
  (params (FaceingLoction :type Vector%20%28by%20ref%29 :default "0, 0, 0"))
  (Class|MotionWarpingComponent|AddorUpdateWarpTargetfromLocation (Variables|Default|GetMotionWarping) "FacingTarget" FaceingLoction))

(event EventSpawnLoot
  ;[1 1 1] 生成掉落物
  (bind _returnvalue (Class|AuraAbilitySystemBPLibary|GetLootTiersInfo self))
  (Utilities|IsValid _returnvalue
    (:Is%20Valid
      (bind _returnvalue_2 (Class|LootTiers|GetLootItems _returnvalue))
      (if (> (Utilities|Array|Length _returnvalue_2) 0)
        (bind _output_get (Variables|Default|SetPureSpawnItem _returnvalue_2))
        (Variables|Default|SetLootRotations (CallFunction|SpawnLootRotaions _output_get))
        (Variables|Default|SetSpawnedLootCount 0)
        (bind _returnvalue_3 (Utilities|Time|SetTimerbyEvent (delegate Custom|SpawnLootItem) 0.05 true))
        (Variables|Default|SetSpawnLootEventHandle _returnvalue_3)
        (CallFunction|SpawnLootItem)))))

(fn ConstructionScript)

(fn SpawnLootRotaions
  (params (TargetArray :type Array%20of%20Loot%20Item%20Structures))
  (return (Class|AuraAbilitySystemBPLibary|EvenlySpeacedRotators (Transformation|GetActorForwardVector) (Math|Vector|VectorUp) 3.6e+02 (Utilities|Array|Length TargetArray))))

(fn GetSpawnTransfrom
  (params (Distance :type Float%20%28single-precision%29))
  (bind _lootrotations (Variables|Default|GetLootRotations))
  (bind _spawnedlootcount (Variables|Default|GetSpawnedLootCount))
  (bind _output (Utilities|Array|Get(acopy) _lootrotations _spawnedlootcount))
  (return (Math|Transform|MakeTransform (+ (* (Math|Vector|GetForwardVector _output) Distance) (Transformation|GetActorLocation)) _output)))