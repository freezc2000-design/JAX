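; Player character Blueprint for Aura, adding facing, shock-state and obstruction-fade hooks.
; A facing event feeds a target location into Motion Warping as the FacingTarget warp target.
; A setter stores the ShockLoop flag; its OnRep function is empty.
; FadeCollision overlaps tell actors implementing BI_FadeInterFace to fade out on entry and back in on exit.
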(event OnComponentBeginOverlap(FadeCollision)
  (params (OverlappedComponent :type Primitive%20Component%20Object%20Reference) (OtherActor :type Actor%20Object%20Reference) (OtherComp :type Primitive%20Component%20Object%20Reference) (OtherBodyIndex :type Integer) (bFromSweep :type Boolean) (SweepResult :type Hit%20Result%20Structure%20%28by%20ref%29))
  (if (Utilities|DoesObjectImplementInterface OtherActor "/Game/Blueprints/Actor/FadeActor/BI_FadeInterFace.BI_FadeInterFace_C")
    (Class|BIFadeInterFace|FadeOut(Message) OtherActor)))

(event OnComponentEndOverlap(FadeCollision)
  (params (OverlappedComponent :type Primitive%20Component%20Object%20Reference) (OtherActor :type Actor%20Object%20Reference) (OtherComp :type Primitive%20Component%20Object%20Reference) (OtherBodyIndex :type Integer))
  (if (Utilities|DoesObjectImplementInterface OtherActor "/Game/Blueprints/Actor/FadeActor/BI_FadeInterFace.BI_FadeInterFace_C")
    (Class|BIFadeInterFace|Fadein(Message) OtherActor)))

(event EventBeginPlay)

(event Collision|EventActorBeginOverlap
  (params (OtherActor :type Actor%20Object%20Reference)))

(event EventTick
  (params (DeltaSeconds :type Float%20%28single-precision%29)))

(event EventSetFaceingTargetLoc
  (params (FaceingLoction :type Vector%20%28by%20ref%29 :default "0, 0, 0"))
  (Class|MotionWarpingComponent|AddorUpdateWarpTargetfromLocation (Variables|Default|GetMotionWarping) "FacingTarget" FaceingLoction))

(event EventSetShockLoop
  (params (bInLoop :type Boolean))
  (Variables|Default|SetbShockLoop bInLoop))

(fn ConstructionScript)

(fn OnRepBShockLoop)