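; GA_VoltBolt is a lightning gameplay ability that fires projectiles toward the target under the mouse, passing the hit actor as homing target.
; On valid target data it turns the avatar toward the hit location via CombatInterface and plays the reused FireBolt cast montage.
; The montage's gameplay event commits the ability and spawns the projectiles with a pitch override.
; The ability ends when the montage completes, blends out, is interrupted or is cancelled.
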(event Ability|EventActivateAbility
  (bind _datahandle (|TargetDataUnderMouse self)
    (:ValidData
      (Variables|Default|SetProjectileTargetLoc (.location (Ability|TargetData|GetHitResultfromTargetData _datahandle)))
      (bind _ascombat_interface (Utilities|Casting|CastToCombatInterface (Ability|GetAvatarActorfromActorInfo)))
      (Class|CombatInterface|SetFaceingTargetLoc _ascombat_interface (Variables|Default|GetProjectileTargetLoc))
      (Variables|Default|SetMouseHitActor (.hitactor (Ability|TargetData|GetHitResultfromTargetData _datahandle)))
      (|PlayMontageandWaitProxy "None" "/Game/Characters/Models/Shared/Aura/Animations/Abilities/AM_Cast_FireBolt.AM_Cast_FireBolt" 1.0 "None" false 1.0 0.0 false
        (:then
          (Ability|Tasks|WaitGameplayEvent "(TagName=\"Event.Montag.FireBolt\")" 0
            (:EventReceived
              (Ability|CommitAbility)
              (Class|AuraFireBolt|SpawnProjectiles (Variables|Default|GetProjectileTargetLoc) false 2e+01 (Variables|Default|GetMouseHitActor)))))
        (:OnCompleted
          (Ability|EndAbility :!label _label))
        (:OnBlendOut
          (goto _label))
        (:OnInterrupted
          (goto _label))
        (:OnCancelled
          (goto _label))))))

(event Ability|EventOnEndAbility
  (params (bWasCancelled :type Boolean)))