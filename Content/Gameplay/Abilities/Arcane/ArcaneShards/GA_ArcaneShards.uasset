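; Arcane Shards gameplay ability: the caster aims with a magic circle, then an input press calls down a series of damaging shards at the cursor's location.
; A spawned BP_PointCollection supplies randomly rotated ground points, their count set by ability level up to a cap.
; After the cast montage, a looping timer fires a gameplay cue and radial damage per point.
; Cooldown commits as shards begin; cost commits after the last, before the ability ends.
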(event Custom|SpawnShard
  (if (< (Variables|Default|GetPointIndex) (Variables|Default|GetNum%20Points))
    (CallFunction|UpdateSpawnLocation)
    (Class|GameplayAbility|ExecuteGameplayCuewithParams "(TagName=\"GameplayCue.ArcaneShards\")" (Ability|GameplayCue|MakeGameplayCueParameters :Location (Variables|Default|GetSpawnLocation)))
    (CallFunction|ApplyDamagetoRadios)
    (else
      (Utilities|Time|ClearandInvalidateTimerbyHandle (Variables|Default|GetSpawnShardHandl))
      (Ability|CommitAbilityCost false)
      (Utilities|FlowControl|Delay 0.2)
      (Ability|EndAbility))))

(event Ability|EventActivateAbility
  (bind _returnvalue (Ability|GetAvatarActorfromActorInfo))
  (Utilities|FlowControl|Sequence
    (:then_0
      (if (Utilities|DoesObjectImplementInterface _returnvalue "/Script/Aura_Learn.CombatInterface")
        (Class|PlayerInterface|ShowMagicCricle(Message) _returnvalue 0)
        (CallFunction|CheckPointComponent)
        (else
          (Ability|CancelAbility))))
    (:then_1
      (Ability|Tasks|WaitInputPress false
        (:OnPress
          (bind _datahandle (|TargetDataUnderMouse)
            (:ValidData
              (Transformation|SetActorLocation (Variables|Default|GetSpawnPoints) (.impactpoint (Ability|TargetData|GetHitResultfromTargetData _datahandle)) false false)
              (Variables|Default|SetNum%20Points (Math|Integer|Min(Integer) (Ability|GetAbilityLevel) (Variables|Default|GetMaxNumArcane)))
              (Variables|Default|SetPointsArray (Class|PointCollection|GetGroundPoints (Variables|Default|GetSpawnPoints) (.impactpoint (Ability|TargetData|GetHitResultfromTargetData _datahandle)) (Variables|Default|GetNum%20Points) (Math|Random|RandomFloatinRange 0.0 3.6e+02)))
              (Variables|Default|SetPointIndex 0)
              (Class|CombatInterface|SetFaceingTargetLoc(Message) (Ability|GetAvatarActorfromActorInfo) (.location (Ability|TargetData|GetHitResultfromTargetData _datahandle)))
              (Class|PlayerInterface|HideMagicCricle(Message) (Ability|GetAvatarActorfromActorInfo))
              (|PlayMontageandWaitProxy "None" "/Game/Characters/Models/Shared/Aura/Animations/Abilities/AM_Cast_ArcaneShards_Short.AM_Cast_ArcaneShards_Short" 1.0 "None" false 1.0 0.0 false
                (:OnCompleted
                  _)
                (:OnBlendOut
                  _)
                (:OnInterrupted
                  _))
              (bind _returnvalue_2 (Utilities|Time|SetTimerbyEvent (delegate Custom|SpawnShard) (Variables|Default|GetSpawnDelta) true))
              (Variables|Default|SetSpawnShardHandl _returnvalue_2)
              (CallFunction|SpawnShard)
              (Ability|CommitAbilityCooldown false))))))))

(event Ability|EventOnEndAbility
  (params (bWasCancelled :type Boolean)))

(fn CheckPointComponent
  (Variables|Default|GetSpawnPoints
    (:then)
    (:else
      (bind _returnvalue (Game|SpawnActorfromClass "/Game/Gameplay/Abilities/Arcane/ArcaneShards/BP_PointCollection.BP_PointCollection_C" (Math|Transform|MakeTransform (Transformation|GetActorLocation (Ability|GetAvatarActorfromActorInfo)) "0, 0, 0" "1.000000,1.000000,1.000000") "AlwaysSpawn" "MultiplyWithRoot" 0 0))
      (Variables|Default|SetSpawnPoints _returnvalue))))

(fn ApplyDamagetoRadios
  (bind _returnvalue (Ability|GetAvatarActorfromActorInfo))
  (bind _outoverlappingactors (Class|AuraAbilitySystemBPLibary|GetLivePlayerswithRadius _returnvalue (Utilities|Array|MakeArray _returnvalue) (Variables|Default|GetSpawnLocation) (Variables|Default|GetRadialDamageOuterRadius)))
  (Variables|Default|SetRadialDamageOrigin (Variables|Default|GetSpawnLocation))
  (for _array_element _outoverlappingactors
    (Class|AuraAbilitySystemBPLibary|ApplyDamageEffect (Class|AuraDamageGameplayAbility|MakeDamageEffectParamsfromClassDefaults _array_element)))
  (Math|Integer|IncrementInt (Variables|Default|GetPointIndex)))

(fn UpdateSpawnLocation
  (Variables|Default|SetSpawnLocation (Transformation|GetWorldLocation (Utilities|Array|Get(acopy) (Variables|Default|GetPointsArray) (Variables|Default|GetPointIndex)))))