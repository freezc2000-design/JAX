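; Battle game mode that applies the selected hero's appearance to the player character when play begins.
; On BeginPlay it reads Y3SelectedHeroIndex from BP_AuraGameInstance and swaps player 0's skeletal mesh to the red, green or blue hero.
; Only the mesh changes, and an unrecognized index or failed game instance cast leaves the character as it is.
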(event EventBeginPlay
  (bind _returnvalue (Game|GetPlayerCharacter 0))
  (bind _mesh (Variables|/Script/Engine.Character|GetMesh _returnvalue))
  (bind _asbp_aura_game_instance (Utilities|Casting|CastToBP_AuraGameInstance (Game|GetGameInstance)))
  (if (== (Variables|/Game/Blueprints/Game/BP_AuraGameInstance.BP_AuraGameInstance_C|GetY3_SelectedHeroIndex _asbp_aura_game_instance) 1)
    (Components|SkeletalMesh|SetSkeletalMeshAsset _mesh "/Game/Characters/Heroes/Demo/Meshes/SKM_Hero_Red.SKM_Hero_Red")
    (elif (== (Variables|/Game/Blueprints/Game/BP_AuraGameInstance.BP_AuraGameInstance_C|GetY3_SelectedHeroIndex _asbp_aura_game_instance) 2)
      (Components|SkeletalMesh|SetSkeletalMeshAsset _mesh "/Game/Characters/Heroes/Demo/Meshes/SKM_Hero_Green.SKM_Hero_Green")
      (elif (== (Variables|/Game/Blueprints/Game/BP_AuraGameInstance.BP_AuraGameInstance_C|GetY3_SelectedHeroIndex _asbp_aura_game_instance) 3)
        (Components|SkeletalMesh|SetSkeletalMeshAsset _mesh "/Game/Characters/Heroes/Demo/Meshes/SKM_Hero_Blue.SKM_Hero_Blue")))))

(event EventTick
  (params (DeltaSeconds :type Float%20%28single-precision%29)))

(fn ConstructionScript)